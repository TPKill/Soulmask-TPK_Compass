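; Mod component that sets up the TPK compass on server and client and removes its widget on EndPlay.
; Servers spawn a single A_TPK_Compass actor if none exists.
; Non-dedicated instances poll on a looping timer, working around a race condition, until WBP_GameMain exists, then add one Wb_TPK_Compass to the viewport linked to this component.
; Code to hide the CanvasPanel_ZhiNanZhen child of the main HUD is disconnected.
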(event `self.ReceiveBeginPlay`
  (bind _returnvalue (`KismetSystemLibrary.IsDedicatedServer`))
  (`/TPK_Compass/TPK_Macros.NOr+Branch` (`KismetSystemLibrary.IsServer`) _returnvalue
    (:`true`
      (bind _returnvalue_2 (`KismetSystemLibrary.K2_SetTimer` null "InitClient" 2.0 true :!label _label))
      (set `self.InitTimer` _returnvalue_2))
    (:`false`
      (`self.InitServer`)
      (if (not _returnvalue)
        (goto _label)))))

(event `self.ReceiveEndPlay`
  (params (EndPlayReason :type "EEndPlayReason Enum" :default "Destroyed"))
  (if (not (`KismetSystemLibrary.IsDedicatedServer`))
    (`self.DestroyClient`)))

(fn `DestroyClient`
  (bind _widget (`self.Widget`))
  (`/Engine/EditorBlueprintResources/StandardMacros.IsValid` _widget
    (:`Is Valid`
      (`Widget.RemoveFromParent` _widget)
      (`/TPK_Compass/UI/HUD/wb_TPK_Compass.Halt` _widget)
      (return))))

(fn `InitClient`
  (bind _foundwidgets (`WidgetBlueprintLibrary.GetAllWidgetsOfClass` "/TPK_Compass/UI/HUD/wb_TPK_Compass.wb_TPK_Compass_C")) ; There seems to be a race condition... so...
  (`/TPK_Compass/TPK_Macros.==+Branch` (`KismetArrayLibrary.Array_Length` _foundwidgets)
    (:`true`
      (bind _foundwidgets_2 (`WidgetBlueprintLibrary.GetAllWidgetsOfClass` "/Game/Blueprints/UI/GameMain/WBP_GameMain.WBP_GameMain_C"))
      (for _array_element _foundwidgets_2
        (for _array_element_2 (`PanelWidget.GetAllChildren` (`HUIGameMain.CanvasPanel_Main` _array_element))
          (if (`KismetStringLibrary.EqualEqual_StrStr` (`KismetSystemLibrary.GetDisplayName` _array_element_2) "CanvasPanel_ZhiNanZhen")
            _))
        (bind _foundwidgets_3 (`WidgetBlueprintLibrary.GetAllWidgetsOfClass` "/TPK_Compass/UI/HUD/wb_TPK_Compass.wb_TPK_Compass_C"))
        (`/TPK_Compass/TPK_Macros.==+Branch` (`KismetArrayLibrary.Array_Length` _foundwidgets_3)
          (:`true`
            (bind _returnvalue (`|CreateWidget` "/TPK_Compass/UI/HUD/wb_TPK_Compass.wb_TPK_Compass_C" (`GameplayStatics.GetPlayerControllerFromID` 0)))
            (bind _output_get (set `self.Widget` _returnvalue))
            (set `/TPK_Compass/UI/HUD/wb_TPK_Compass.ModAC` self _output_get)
            (`UserWidget.AddToViewport` _output_get 0))))
      (return))
    (:`false`
      (`KismetSystemLibrary.K2_ClearAndInvalidateTimerHandle` (`self.InitTimer`))
      (return))))

(fn `InitServer`
  (bind _outactors (`GameplayStatics.GetAllActorsOfClass` "/TPK_Compass/a_TPK_Compass.a_TPK_Compass_C"))
  (`/TPK_Compass/TPK_Macros.==+Branch` (`KismetArrayLibrary.Array_Length` _outactors)
    (:`true`
      (`|SpawnActorFromClass` "/TPK_Compass/a_TPK_Compass.a_TPK_Compass_C" (`KismetMathLibrary.MakeTransform` (0.0 0.0 10000.0)) "AlwaysSpawn" "OverrideRootScale" null null)
      (return))))